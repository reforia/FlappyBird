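; Flappy Bird-style player pawn driven by physics on its Bird component.
; Each tick applies a constant vertical acceleration (FallingSpeed), and a tap press overrides linear velocity with an upward boost.
; Tilt is set through roll, held at one extreme while rising and interpolated toward the other as downward speed approaches the boost magnitude.
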(event EventBeginPlay)

(event Collision|EventActorBeginOverlap
  (params (OtherActor :type Actor%20Object%20Reference)))

(event EventTick
  (params (DeltaSeconds :type Float%20%28single-precision%29))
  (bind _tapboostforce (Variables|Default|GetTapBoostForce))
  (bind _maxrotationpitchangle (Variables|Default|GetMaxRotationPitchAngle))
  (Physics|AddForce (Variables|Default|GetBird) (Math|Vector|MakeVector 0.0 0.0 (Variables|Default|GetFallingSpeed)) "None" true)
  (Transformation|SetRelativeRotation (Variables|Default|GetBird) (Math|Rotator|MakeRotator (Math|Float|Lerp (* _maxrotationpitchangle -1.0) _maxrotationpitchangle (Math|Float|Absolute(Float) (Math|Float|Min(Float) (/ (Math|Float|Clamp(Float) (.z (Transformation|GetComponentVelocity (Variables|Default|GetBird))) (* _tapboostforce -1.0) _tapboostforce) _tapboostforce) 0.0))) 0.0 0.0) false false))

(event EventOnTap
  (params (IsPreesed :type Boolean))
  (if IsPreesed
    (Physics|SetPhysicsLinearVelocity (Variables|Default|GetBird) (Math|Vector|MakeVector 0.0 0.0 (Variables|Default|GetTapBoostForce)) false "None")))

(fn ConstructionScript)