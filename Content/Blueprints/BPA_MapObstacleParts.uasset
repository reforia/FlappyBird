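; Obstacle actor with top and bottom parts separated by a gap the player passes through to score.
; InitializeGap randomizes the bottom part's height within the given range and offset, then places the top part one clamped gap above it.
; A pawn overlapping either part's collision reports a crash to the game mode, while leaving the Bound volume awards a point.
; Both notifications reach the game mode as interface messages.
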(event OnComponentBeginOverlap(BottomCollision)
  (params (OverlappedComponent :type Primitive%20Component%20Object%20Reference) (OtherActor :type Actor%20Object%20Reference) (OtherComp :type Primitive%20Component%20Object%20Reference) (OtherBodyIndex :type Integer) (bFromSweep :type Boolean) (SweepResult :type Hit%20Result%20Structure%20%28by%20ref%29))
  (Utilities|Casting|CastToPawn OtherActor)
  (CallFunction|PlayerCrashed))

(event OnComponentBeginOverlap(TopCollision)
  (params (OverlappedComponent :type Primitive%20Component%20Object%20Reference) (OtherActor :type Actor%20Object%20Reference) (OtherComp :type Primitive%20Component%20Object%20Reference) (OtherBodyIndex :type Integer) (bFromSweep :type Boolean) (SweepResult :type Hit%20Result%20Structure%20%28by%20ref%29))
  (Utilities|Casting|CastToPawn OtherActor)
  (CallFunction|PlayerCrashed))

(event OnComponentEndOverlap(Bound)
  (params (OverlappedComponent :type Primitive%20Component%20Object%20Reference) (OtherActor :type Actor%20Object%20Reference) (OtherComp :type Primitive%20Component%20Object%20Reference) (OtherBodyIndex :type Integer))
  (Utilities|Casting|CastToPawn OtherActor)
  (Class|BPIGameplayUtil|OnPlayerGainPoint(Message) (Game|GetGameMode) 1))

(event Custom|InitializeGap
  (params (Gap :type Float%20%28double-precision%29) (MinHeight :type Float%20%28double-precision%29) (MaxHeight :type Float%20%28double-precision%29) (ZOffset :type Float%20%28double-precision%29))
  (bind _returnvalue (- MaxHeight MinHeight))
  (bind _bottomroot (Variables|Default|GetBottomRoot))
  (bind _returnvalue_2 (Math|Float|Clamp(Float) Gap 0.0 _returnvalue))
  (Transformation|SetRelativeLocation _bottomroot (Math|Vector|MakeVector 0.0 0.0 (- (Math|Random|RandomFloatinRange 1e+01 (- _returnvalue _returnvalue_2)) ZOffset)) false true)
  (Transformation|SetRelativeLocation (Variables|Default|GetTopRoot) (Math|Vector|MakeVector 0.0 0.0 (+ (.z (Variables|/Script/Engine.SceneComponent|GetRelativeLocation _bottomroot)) _returnvalue_2)) false true))

(event Custom|PlayerCrashed
  (Class|BPIGameplayUtil|OnPlayerCrashed(Message) (Game|GetGameMode)))

(event EventBeginPlay)

(event Collision|EventActorBeginOverlap
  (params (OtherActor :type Actor%20Object%20Reference)))

(event EventTick
  (params (DeltaSeconds :type Float%20%28single-precision%29)))

(fn ConstructionScript)