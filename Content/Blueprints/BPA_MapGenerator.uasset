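; Map generator actor for a Flappy Bird game that keeps a scrolling row of obstacle parts going.
; On the game mode's initialization event it spawns ten parts spaced by SpawnGap, each initialized with gap and height-range settings.
; A looping timer, rather than Tick, shifts every part along Y at MapPanSpeed.
; Parts overlapping the Box trigger are destroyed and replaced by a new one placed relative to the last.
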(event OnComponentBeginOverlap(Box)
  (params (OverlappedComponent :type Primitive%20Component%20Object%20Reference) (OtherActor :type Actor%20Object%20Reference) (OtherComp :type Primitive%20Component%20Object%20Reference) (OtherBodyIndex :type Integer) (bFromSweep :type Boolean) (SweepResult :type Hit%20Result%20Structure%20%28by%20ref%29))
  (if (Utilities|IsValid OtherActor)
    (bind _asbpa_map_obstacle_parts (Utilities|Casting|CastToBPA_MapObstacleParts OtherActor))
    (CallFunction|RemoveandRefillBlocks _asbpa_map_obstacle_parts)))

(event Custom|InitializeObstacles
  (for _index (range 0 9)
    (CallFunction|GenerateBlocks (Variables|Default|GetSpawnGap)))
  (bind _returnvalue (Utilities|Time|SetTimerbyEvent (delegate Custom|UpdateParts) 0.016 true))
  (Variables|Default|SetPartsUpdateTimerHandle _returnvalue))

(event Custom|UpdateParts
  (for _array_element (Variables|Default|GetPartsArray)
    (Transformation|AddActorLocalOffset _array_element (Math|Vector|MakeVector 0.0 (* (Variables|Default|GetMapPanSpeed) -1.0) 0.0) false false)))

(event EventBeginPlay
  (bind _asgm_flappy_bird (Utilities|Casting|CastToGM_FlappyBird (Game|GetGameMode)))
  (EventDispatchers|BindEventtoOnGameInitialization _asgm_flappy_bird (delegate Custom|InitializeObstacles)))

(event Collision|EventActorBeginOverlap
  (params (OtherActor :type Actor%20Object%20Reference)))

(event EventTick
  (params (DeltaSeconds :type Float%20%28single-precision%29)))

(fn ConstructionScript)

(fn GenerateBlocks
  (params (SpawnGap :type Float%20%28double-precision%29))
  (bind _partsarray (Variables|Default|GetPartsArray))
  (bind _returnvalue (Utilities|Array|Length _partsarray))
  (if (> _returnvalue 0)
    (LocalVariables|SetNewBlockLocation (- (Transformation|GetActorLocation (Utilities|Array|Get(acopy) _partsarray (- _returnvalue 1))) (* (Math|Vector|GetRightVector (Variables|Default|GetLeftMostActorStartPoint)) SpawnGap)))
    (else
      (LocalVariables|SetNewBlockLocation (Transformation|GetWorldLocation (Variables|Default|GetLeftMostActorStartPoint)))))
  (bind _returnvalue_2 (Game|SpawnActorfromClass "/Game/Blueprints/BPA_MapObstacleParts.BPA_MapObstacleParts_C" (Math|Transform|MakeTransform (LocalVariables|GetNewBlockLocation) "0, 0, 0" "1.000000,1.000000,1.000000") "Undefined" 0 0))
  (Default|InitializeGap _returnvalue_2 3e+02 -4e+02 4e+02 3e+02)
  (Utilities|Array|AddUnique (Variables|Default|GetPartsArray) _returnvalue_2)
  (Transformation|AttachComponentToComponent _returnvalue_2 (Variables|Default|GetParts) "None" "KeepWorld" "KeepWorld" "KeepWorld" true))

(fn RemoveandRefillBlocks
  (params (PartReference :type BPA%20Map%20Obstacle%20Parts%20Object%20Reference))
  (if (Utilities|Array|ContainsItem (Variables|Default|GetPartsArray) PartReference)
    (Utilities|Array|RemoveItem (Variables|Default|GetPartsArray) PartReference))
  (Actor|DestroyActor PartReference)
  (CallFunction|GenerateBlocks (Variables|Default|GetSpawnGap)))